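; BP_KA_ProjectileTest is an AK rifle weapon that fires projectiles for players and bots, with optional sight and vertical grip.
; Gates for draw delay and trigger feed a firing chain that plays sound, adds camera shake and recoil, and spawns projectiles.
; Spread grows by timeline per shot and recovers on Tick; CalculateSpray scales it by movement, crouch and aim.
; Projectile hits route damage to the server and impact effects through multicast.
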(event `self.PickUp`
  (bind _returnvalue (/ 0.1 -20.0))
  (bind _returnvalue_2 (/ 0.8 -15.0))
  (bind _player (`self.player`))
  (bind _player_2 (`self.player`))
  (bind _player_3 (`self.player`))
  (bind _startspray (`self.startSpray`))
  (bind _player_4 (`self.player`))
  (bind _returnvalue_3 (`Pawn.IsBotControlled` _player_3))
  (set `self.drawing` true)
  (`|ExecutionSequence`
    (:`then_0`
      (`KismetSystemLibrary.Delay` 0.1)
      (set `self.drawing` false)
      (`KismetSystemLibrary.Delay` 0.4)
      (goto _label :!via `Open`))
    (:`then_1`
      (goto _label :!via `Close`))))

(event `self.Shoot`
  (bind _returnvalue (/ 0.1 -20.0))
  (bind _returnvalue_2 (/ 0.8 -15.0))
  (bind _player (`self.player`))
  (bind _player_2 (`self.player`))
  (bind _player_3 (`self.player`))
  (bind _startspray (`self.startSpray`))
  (bind _player_4 (`self.player`))
  (bind _returnvalue_3 (`Pawn.IsBotControlled` _player_3))
  ;[1 1 1] can I shoot?
  (`/Engine/EditorBlueprintResources/StandardMacros.Gate` true :!label _label
    (:`Exit`
      (`/Engine/EditorBlueprintResources/StandardMacros.Gate` true :!label _label_2
        (:`Exit`
          (`/Engine/EditorBlueprintResources/StandardMacros.IsValid` (`self.player`)
            (:`Is Valid`
              (if (and (`KismetMathLibrary.Conv_IntToBool` (`self.InClip`)) (not (`/Game/MultiplayerShooterEngine/Blueprints/BP_PlayerBase.reloading` _player)) (== (`/Game/MultiplayerShooterEngine/Blueprints/BP_PlayerBase.runProgres` _player) 0.0))
                (set `self.shooting_animation` true)
                (`KismetSystemLibrary.Delay` (`self.shootDelay`))
                (if (and (`Pawn.IsLocallyControlled` _player_3) (not _returnvalue_3))
                  (`GameplayStatics.PlaySound2D` "/Game/MultiplayerShooterEngine/Sounds/Rifle_Fire_Cue.Rifle_Fire_Cue" 0.5 0.9 0.0 null null false)
                  (bind _asplayer_controller (cast `PlayerController` (`Pawn.GetController` (`self.player`)) :!label _label_3)
                    (:`then`
                      (`self.PlayShotSoundServer`)
                      (if (> (`/Game/MultiplayerShooterEngine/Blueprints/BP_PlayerBase.aim` (`self.player`)) 0.7)
                        (`PlayerController.ClientStartCameraShake` :`self` _asplayer_controller :`Shake` "/Game/MultiplayerShooterEngine/Blueprints/Weapons/AK/WeaponCameraShake.WeaponCameraShake_C" :`Scale` 0.2)
                        ;[1 1 1] reloil
                        (`Pawn.AddControllerPitchInput` _player_4 (`KismetMathLibrary.SelectFloat` -0.1 -0.11 (`self.Vertgrip`)))
                        (`Pawn.AddControllerYawInput` _player_4 (`KismetMathLibrary.RandomFloatInRange` (* _returnvalue_2 -1.0) _returnvalue_2))
                        (else
                          (`PlayerController.ClientStartCameraShake` :`self` _asplayer_controller :`Shake` "/Game/MultiplayerShooterEngine/Blueprints/Weapons/AK/WeaponCameraShake.WeaponCameraShake_C" :`Scale` 0.5)
                          (`Pawn.AddControllerPitchInput` _player_2 (`KismetMathLibrary.SelectFloat` -0.05 -0.04 (`self.Vertgrip`)))
                          (`Pawn.AddControllerYawInput` _player_2 (`KismetMathLibrary.RandomFloatInRange` (* _returnvalue -1.0) _returnvalue)))))
                    (:`CastFailed`
                      _))
                  (bind _output_get (set `self.InClip` (- (stale _output_get) 1)))
                  (`self.SpawnProjectile`)
                  (set `self.startSpray` (`self.spread`))
                  (`|ExecutionSequence`
                    (:`then_0`
                      (`|ExecutionSequence`
                        (:`then_0`
                          (`KismetSystemLibrary.RetriggerableDelay` 0.2)
                          (goto _label_4 :!via `Open`))
                        (:`then_1`
                          (goto _label_4 :!via `Close`))))
                    (:`then_1`
                      (bind (_direction _newtrack_0) (`Timeline|SmoothSpray` :!via `PlayFromStart`)
                        (:`Update`
                          (set `self.spread` (`KismetMathLibrary.FClamp` (`KismetMathLibrary.Lerp` _startspray (+ _startspray (`KismetMathLibrary.SelectFloat` 4.0 3.0 (`self.Vertgrip`))) _newtrack_0) 0.0 (`KismetMathLibrary.SelectFloat` 40.0 20.0 (`self.Vertgrip`))))))))
                  (elif _returnvalue_3
                    (`self.PlayShot`)
                    (goto _label_3)))
                (else
                  (set `self.shooting_animation` false))))))))))

(event `SprayReset`
  (`/Engine/EditorBlueprintResources/StandardMacros.Gate` true :!label _label_4
    (:`Exit`
      (bind _output_get (set `self.spread` (`KismetMathLibrary.FClamp` (- (stale _output_get) (* (`GameplayStatics.GetWorldDeltaSeconds`) 100.0)) 0.0 60.0))))))

(event `self.LMBPressed`
  ;[1 1 1] can I shoot?
  (goto _label_2 :!via `Open`))

(event `self.LMBReleased`
  ;[1 1 1] can I shoot?
  (`|ExecutionSequence`
    (:`then_0`
      (goto _label_2 :!via `Close`))
    (:`then_1`
      (set `self.shooting_animation` false))))

(event `PlayShot`
  (bind _player (`self.player`))
  (`/Engine/EditorBlueprintResources/StandardMacros.IsValid` _player
    (:`Is Valid`
      (if (`Pawn.IsLocallyControlled` _player)
        (if (`Pawn.IsBotControlled` _player)
          (`GameplayStatics.PlaySoundAtLocation` "/Game/MultiplayerShooterEngine/Sounds/Rifle_Fire_Cue.Rifle_Fire_Cue" (`self.K2_GetActorLocation`) (struct) 0.8 1.0 0.0 null null null null :!label _label_5)
          (set `self.shooting_animation` true)
          (`KismetSystemLibrary.RetriggerableDelay` 0.3)
          (set `self.shooting_animation` false))
        (else
          (goto _label_5))))))

(event `self.ReceiveBeginPlay`
  (`parent.ReceiveBeginPlay`))

(event `PlayShotSoundServer`
  (`self.PlayShot`))

(event `self.ReceiveTick`
  (params (DeltaSeconds :type "Float (single-precision)"))
  (bind _weapon (`self.Weapon`))
  (bind _player (`self.player`))
  (bind _childactor (`ChildActorComponent.ChildActor` (`self.ChildActor`)))
  (`parent.ReceiveTick` DeltaSeconds)
  (`|ExecutionSequence`
    (:`then_0`
      (`self.ProjectileSpawnUpdate`)
      (`self.SprayReset`)
      (if (`KismetSystemLibrary.IsValid` (`self.player`))
        (`PrimitiveComponent.SetCastShadow` _weapon (not (`Pawn.IsLocallyControlled` (`self.player`))))
        (`PrimitiveComponent.SetCastShadow` (`self.SM_T4_Sight`) (not (`Pawn.IsLocallyControlled` (`self.player`))))
        (`PrimitiveComponent.SetCastShadow` (`self.SM_Vertgrip`) (not (`Pawn.IsLocallyControlled` (`self.player`))))
        (bind _asbp_sight_lense (cast `/Game/MultiplayerShooterEngine/Blueprints/BP_SightLense` _childactor))
        (set `/Game/MultiplayerShooterEngine/Blueprints/BP_SightLense.enabled` (and (== (`/Game/MultiplayerShooterEngine/Blueprints/BP_PlayerBase.Weapon_BP` _player) self) (`Pawn.IsLocallyControlled` _player) (> (`/Game/MultiplayerShooterEngine/Blueprints/BP_PlayerBase.aim` _player) 0.3)) _asbp_sight_lense)
        (else
          (`PrimitiveComponent.SetCastShadow` _weapon true)
          (`PrimitiveComponent.SetCastShadow` (`self.SM_T4_Sight`) true)
          (`PrimitiveComponent.SetCastShadow` (`self.SM_Vertgrip`) true)
          (bind _asbp_sight_lense_2 (cast `/Game/MultiplayerShooterEngine/Blueprints/BP_SightLense` _childactor))
          (set `/Game/MultiplayerShooterEngine/Blueprints/BP_SightLense.enabled` false _asbp_sight_lense_2))))
    (:`then_1`
      (`SceneComponent.SetVisibility` (`self.SM_Vertgrip`) (`self.Vertgrip`) false))))

(fn `CalculateSpray`
  (returns (spray :type "Float (double-precision)"))
  (bind _player (`self.player`))
  (`/Engine/EditorBlueprintResources/StandardMacros.IsValid` _player
    (:`Is Valid`
      (return (`KismetMathLibrary.Lerp` (* (+ (* (`self.spread`) 1.3) (* (`KismetMathLibrary.VSize` (`self.GetVelocity` _player)) 0.05) (`KismetMathLibrary.SelectFloat` 7.0 10.0 (`NavMovementComponent.IsCrouching` (`Character.CharacterMovement` _player)))) 0.7) 0.0 (`/Game/MultiplayerShooterEngine/Blueprints/BP_PlayerBase.aim` _player))))))

(fn `Projectile Hited`
  (params (hit :type "HitResult Structure"))
  (bind (_bblockinghit _binitialoverlap _time _distance _location _impactpoint _normal _impactnormal _physmat _hitactor _hitcomponent _hitbonename) (`GameplayStatics.BreakHitResult` hit))
  (if (!= _hitactor (`self.player`))
    ;[1 1 1] hit
    (`|ExecutionSequence`
      (:`then_0`
        (`/Game/MultiplayerShooterEngine/Blueprints/BP_PlayerBase.DamageServer` (`self.player`) _hitactor (`self.damage`) (`KismetStringLibrary.Conv_NameToString` _hitbonename) null self))
      (:`then_1`
        (if _bblockinghit
          (`/Game/MultiplayerShooterEngine/Blueprints/BP_PlayerBase.BulletHitMulticast` (`self.player`) _impactpoint _impactnormal _physmat _hitcomponent))))))

(fn `UserConstructionScript`
  (`parent.UserConstructionScript`)
  (if (`self.sight`)
    (set `self.AimCameraLocation` (-10.21 9.0 -16.049999))
    (else
      (set `self.AimCameraLocation` (-13.4 12.0 -16.07))))
  (`SceneComponent.SetVisibility` (`self.SM_T4_Sight`) (`self.sight`) true))