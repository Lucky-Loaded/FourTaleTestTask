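; AK rifle weapon Blueprint for a multiplayer shooter, with optional sight and vertical grip attachments.
; Draw and trigger gates pass shots to a camera line trace that drives damage, impacts, shell ejection and muzzle flash through the owning Player.
; Timeline-grown spread decays after firing and combines with movement, stance and aim, while grip and aim shape recoil.
; Tick toggles local-only scope and shadows, and repositions the muzzle spawn point to correct first-person scale.
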(event `SprayReset`
  (`/Engine/EditorBlueprintResources/StandardMacros.Gate` true :!label _label
    (:`Exit`
      (bind _output_get (set `self.spread` (`KismetMathLibrary.FClamp` (- (stale _output_get) (* (`GameplayStatics.GetWorldDeltaSeconds`) 100.0)) 0.0 60.0))))))

(event `self.PickUp`
  (bind _returnvalue (/ 0.1 -10.0))
  (bind _returnvalue_2 (/ 0.8 -15.0))
  (bind _player (`self.player`))
  (bind _player_2 (`self.player`))
  (bind _shell (`self.shell`))
  (bind _player_3 (`self.player`))
  (bind _startspray (`self.startSpray`))
  (bind _player_4 (`self.player`))
  (bind _returnvalue_3 (`Pawn.GetControlRotation` _player_3))
  (bind _camera1 (`/Game/MultiplayerShooterEngine/Blueprints/BP_PlayerBase.Camera1` _player_3))
  (set `self.drawing` true)
  (`|ExecutionSequence`
    (:`then_0`
      (`KismetSystemLibrary.Delay` 0.1)
      (set `self.drawing` false)
      (`KismetSystemLibrary.Delay` 0.4)
      (goto _label_2 :!via `Open`))
    (:`then_1`
      (goto _label_2 :!via `Close`))))

(event `self.Shoot`
  (bind _returnvalue (/ 0.1 -10.0))
  (bind _returnvalue_2 (/ 0.8 -15.0))
  (bind _player (`self.player`))
  (bind _player_2 (`self.player`))
  (bind _shell (`self.shell`))
  (bind _player_3 (`self.player`))
  (bind _startspray (`self.startSpray`))
  (bind _player_4 (`self.player`))
  (bind _returnvalue_3 (`Pawn.GetControlRotation` _player_3))
  (bind _camera1 (`/Game/MultiplayerShooterEngine/Blueprints/BP_PlayerBase.Camera1` _player_3))
  ;[1 1 1] can I shoot?
  (`/Engine/EditorBlueprintResources/StandardMacros.Gate` true :!label _label_2
    (:`Exit`
      (`/Engine/EditorBlueprintResources/StandardMacros.Gate` true :!label _label_3
        (:`Exit`
          (`/Engine/EditorBlueprintResources/StandardMacros.IsValid` (`self.player`)
            (:`Is Valid`
              (if (and (`KismetMathLibrary.Conv_IntToBool` (`self.InClip`)) (not (`/Game/MultiplayerShooterEngine/Blueprints/BP_PlayerBase.reloading` _player)) (== (`/Game/MultiplayerShooterEngine/Blueprints/BP_PlayerBase.runProgres` _player) 0.0))
                (set `self.shooting_animation` true)
                (`KismetSystemLibrary.Delay` (`self.shootDelay`))
                (if (`Pawn.IsLocallyControlled` (`self.player`))
                  (`GameplayStatics.PlaySound2D` "/Game/MultiplayerShooterEngine/Sounds/Rifle_Fire_Cue.Rifle_Fire_Cue" 0.5 0.9 0.0 null null false)
                  (bind _asplayer_controller (cast `PlayerController` (`Pawn.GetController` (`self.player`)))
                    (:`then`
                      (`self.PlayShotSoundServer`)
                      (if (> (`/Game/MultiplayerShooterEngine/Blueprints/BP_PlayerBase.aim` (`self.player`)) 0.7)
                        (`PlayerController.ClientStartCameraShake` :`self` _asplayer_controller :`Shake` "/Game/MultiplayerShooterEngine/Blueprints/Weapons/AK/WeaponCameraShake.WeaponCameraShake_C" :`Scale` 0.2)
                        ;[1 1 1] reloil
                        (`Pawn.AddControllerPitchInput` _player_4 (`KismetMathLibrary.SelectFloat` -0.1 -0.11 (`self.Vertgrip`)))
                        (`Pawn.AddControllerYawInput` _player_4 (`KismetMathLibrary.RandomFloatInRange` (* _returnvalue_2 -1.0) _returnvalue_2))
                        (else
                          (`PlayerController.ClientStartCameraShake` :`self` _asplayer_controller :`Shake` "/Game/MultiplayerShooterEngine/Blueprints/Weapons/AK/WeaponCameraShake.WeaponCameraShake_C" :`Scale` 0.5)
                          (`Pawn.AddControllerPitchInput` _player_2 (`KismetMathLibrary.SelectFloat` -0.1 -0.14 (`self.Vertgrip`)))
                          (`Pawn.AddControllerYawInput` _player_2 (`KismetMathLibrary.RandomFloatInRange` (* _returnvalue -1.0) _returnvalue)))))
                    (:`CastFailed`
                      _))
                  (bind _outhit (`KismetSystemLibrary.LineTraceSingle` (`SceneComponent.K2_GetComponentLocation` _camera1) (+ (`SceneComponent.K2_GetComponentLocation` _camera1) (* (`KismetMathLibrary.GetForwardVector` _returnvalue_3) 100000.0) (* (* (`KismetMathLibrary.GreaterGreater_VectorRotator` (`self.randomVector` (- (`self.CalculateSpray`) 5.0)) _returnvalue_3) 100.0) (`KismetMathLibrary.Conv_BoolToDouble` (not (> (`/Game/MultiplayerShooterEngine/Blueprints/BP_PlayerBase.aim` (`self.player`)) 0.2))))) "TraceTypeQuery1" true (`|MakeArray` (`self.player`) :!type "Actor Object Reference") "None" true (struct :`G` 0.076852 :`B` 1.0 :`A` 1.0)))
                  (bind _output_get (set `self.InClip` (- (stale _output_get) 1)))
                  ;[1 1 1] hit
                  (`|ExecutionSequence`
                    (:`then_0`
                      (set `self.startSpray` (`self.spread`))
                      (`|ExecutionSequence`
                        (:`then_0`
                          (`|ExecutionSequence`
                            (:`then_0`
                              (`KismetSystemLibrary.RetriggerableDelay` 0.2)
                              (goto _label :!via `Open`))
                            (:`then_1`
                              (goto _label :!via `Close`))))
                        (:`then_1`
                          (bind (_direction _newtrack_0) (`Timeline|SmoothSpray` :!via `PlayFromStart`)
                            (:`Update`
                              (set `self.spread` (`KismetMathLibrary.FClamp` (`KismetMathLibrary.Lerp` _startspray (+ _startspray (`KismetMathLibrary.SelectFloat` 4.0 3.0 (`self.Vertgrip`))) _newtrack_0) 0.0 (`KismetMathLibrary.SelectFloat` 40.0 20.0 (`self.Vertgrip`)))))))))
                    (:`then_1`
                      (`/Game/MultiplayerShooterEngine/Blueprints/BP_PlayerBase.Damage` (`self.player`) (`.HitActor` (`GameplayStatics.BreakHitResult` _outhit)) (`self.damage`) (`KismetStringLibrary.Conv_NameToString` (`.HitBoneName` (`GameplayStatics.BreakHitResult` _outhit))) (`Pawn.GetController` (`self.player`)) self)
                      (bind _returnvalue_4 (`|SpawnActorFromClass` "/Game/MultiplayerShooterEngine/Blueprints/Weapon/BP_Shell.BP_Shell_C" (`SceneComponent.K2_GetComponentToWorld` _shell) "Undefined" "OverrideRootScale" null null))
                      (`PrimitiveComponent.AddImpulse` (`/Game/MultiplayerShooterEngine/Blueprints/Weapon/BP_Shell.Shell` _returnvalue_4) (+ (* (`SceneComponent.GetForwardVector` _shell) 130.0) (* (`self.GetVelocity` (`self.player`)) 0.5)) "None" false)
                      (`GameplayStatics.SpawnEmitterAttached` null (`self.Muzzle`) "None" (0.0 0.0 0.0) (struct) (1.0 1.0 1.0) "SnapToTargetIncludingScale" true "AutoRelease"))
                    (:`then_2`
                      (if (`GameplayStatics.BreakHitResult` _outhit)
                        (`/Game/MultiplayerShooterEngine/Blueprints/BP_PlayerBase.Hit` (`self.player`) (`.Location` (`GameplayStatics.BreakHitResult` _outhit)) (`.Normal` (`GameplayStatics.BreakHitResult` _outhit)) (`.PhysMat` (`GameplayStatics.BreakHitResult` _outhit)) (`.HitComponent` (`GameplayStatics.BreakHitResult` _outhit)))))))
                (else
                  (set `self.shooting_animation` false))))))))))

(event `self.LMBPressed`
  ;[1 1 1] can I shoot?
  (goto _label_3 :!via `Open`))

(event `self.LMBReleased`
  ;[1 1 1] can I shoot?
  (`|ExecutionSequence`
    (:`then_0`
      (goto _label_3 :!via `Close`))
    (:`then_1`
      (set `self.shooting_animation` false))))

(event `PlayShot`
  (bind _player (`self.player`))
  (`/Engine/EditorBlueprintResources/StandardMacros.IsValid` _player
    (:`Is Valid`
      (if (not (`Pawn.IsLocallyControlled` _player))
        (`GameplayStatics.PlaySoundAtLocation` "/Game/MultiplayerShooterEngine/Sounds/Rifle_Fire_Cue.Rifle_Fire_Cue" (`self.K2_GetActorLocation`) (struct) 0.8 1.0 0.0 "/Game/MultiplayerShooterEngine/Blueprints/BP_HitSound.BP_HitSound" null null null)
        (set `self.shooting_animation` true)
        (`KismetSystemLibrary.RetriggerableDelay` 0.3)
        (set `self.shooting_animation` false)))))

(event `self.ReceiveBeginPlay`
  (`parent.ReceiveBeginPlay`))

(event `PlayShotSoundServer`
  (`self.PlayShot`))

(event `self.ReceiveTick`
  (params (DeltaSeconds :type "Float (single-precision)"))
  (bind _weapon (`self.Weapon`))
  (bind _childactor (`self.ChildActor`))
  (bind _player (`self.player`))
  (bind _returnvalue (`Pawn.IsLocallyControlled` _player))
  (bind _childactor_2 (`ChildActorComponent.ChildActor` _childactor))
  (`parent.ReceiveTick` DeltaSeconds)
  (`|ExecutionSequence`
    (:`then_0`
      (`self.SprayReset`)
      (if (`KismetSystemLibrary.IsValid` (`self.player`))
        (`PrimitiveComponent.SetCastShadow` _weapon (not (`Pawn.IsLocallyControlled` (`self.player`))))
        (`PrimitiveComponent.SetCastShadow` (`self.SM_T4_Sight`) (not (`Pawn.IsLocallyControlled` (`self.player`))))
        (`PrimitiveComponent.SetCastShadow` (`self.SM_Vertgrip`) (not (`Pawn.IsLocallyControlled` (`self.player`))))
        (`/Engine/EditorBlueprintResources/StandardMacros.IsValid` _childactor
          (:`Is Valid`
            (bind _asbp_sight_lense (cast `/Game/MultiplayerShooterEngine/Blueprints/BP_SightLense` _childactor_2))
            (set `/Game/MultiplayerShooterEngine/Blueprints/BP_SightLense.enabled` (and (== (`/Game/MultiplayerShooterEngine/Blueprints/BP_PlayerBase.Weapon_BP` _player) self) _returnvalue (> (`/Game/MultiplayerShooterEngine/Blueprints/BP_PlayerBase.aim` _player) 0.3)) _asbp_sight_lense)
            (`SceneComponent.SetVisibility` (`self.ChildActor`) _returnvalue false)))
        (else
          (`PrimitiveComponent.SetCastShadow` _weapon true)
          (`PrimitiveComponent.SetCastShadow` (`self.SM_T4_Sight`) true)
          (`PrimitiveComponent.SetCastShadow` (`self.SM_Vertgrip`) true)
          (`/Engine/EditorBlueprintResources/StandardMacros.IsValid` _childactor
            (:`Is Valid`
              (bind _asbp_sight_lense_2 (cast `/Game/MultiplayerShooterEngine/Blueprints/BP_SightLense` _childactor_2))
              (`/Engine/EditorBlueprintResources/StandardMacros.IsValid` _asbp_sight_lense_2
                (:`Is Valid`
                  (set `/Game/MultiplayerShooterEngine/Blueprints/BP_SightLense.enabled` false _asbp_sight_lense_2))))))))
    (:`then_1`
      (`SceneComponent.SetVisibility` (`self.SM_Vertgrip`) (`self.Vertgrip`) false))
    (:`then_2`
      ;[1 1 1] Add these function and components to your weapon to fix muzzle scale problems
      ; Also set your weapon tick group to last
      (`self.Update Muzzle Spawn Point` (`self.MuzzleLocation`) (`self.MuzzleSpawnPoint`)))))

(fn `CalculateSpray`
  (returns (spray :type "Float (double-precision)"))
  (bind _player (`self.player`))
  (`/Engine/EditorBlueprintResources/StandardMacros.IsValid` _player
    (:`Is Valid`
      (return (`KismetMathLibrary.Lerp` (* (+ (* (`self.spread`) 1.3) (* (`KismetMathLibrary.VSize` (`self.GetVelocity` _player)) 0.05) (`KismetMathLibrary.SelectFloat` 7.0 10.0 (`NavMovementComponent.IsCrouching` (`Character.CharacterMovement` _player)))) 0.7) 0.0 (`/Game/MultiplayerShooterEngine/Blueprints/BP_PlayerBase.aim` _player))))))

(fn `Update Muzzle Spawn Point`
  (params (Location :type "SceneComponent Object Reference") (`Spawn Point` :type "SceneComponent Object Reference") (Scale :type "Float (double-precision)" :default 0.16))
  (bind _spawn_point (`local.Spawn Point`))
  (bind _returnvalue (`PlayerCameraManager.GetCameraLocation` (`GameplayStatics.GetPlayerCameraManager` 0)))
  (bind _returnvalue_2 (`SceneComponent.K2_GetComponentLocation` (`local.Location`)))
  (bind _player (`self.player`)
    (:`then`
      (if (and (`Pawn.IsLocallyControlled` _player) (not (`Pawn.IsBotControlled` _player)))
        (`SceneComponent.K2_SetWorldLocation` _spawn_point (+ (* (/ (`KismetMathLibrary.Vector_Distance` _returnvalue _returnvalue_2) (`local.Scale`)) (`KismetMathLibrary.GetForwardVector` (`KismetMathLibrary.FindLookAtRotation` _returnvalue _returnvalue_2))) _returnvalue_2) false false)
        (`SceneComponent.SetWorldScale3D` _spawn_point (1.0 1.0 1.0))))
    (:`else`)))

(fn `UserConstructionScript`
  (`parent.UserConstructionScript`)
  (if (`self.sight`)
    (set `self.AimCameraLocation` (-10.007731 16.178574 -16.049999))
    (else
      (set `self.AimCameraLocation` (-13.4 12.0 -16.07))))
  (`SceneComponent.SetVisibility` (`self.SM_T4_Sight`) (`self.sight`) true))