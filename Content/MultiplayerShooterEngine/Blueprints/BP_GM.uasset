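; Game mode for a two-team shooter deathmatch with timed matches, scoring and respawns.
; Joining players are balanced across teams and spawned at random team-tagged PlayerStarts with two starting weapons.
; Deaths update player and team scores, broadcast a kill feed and trigger respawn.
; Tick rebuilds both bubble-sorted team scoreboards and advances the timer, which announces the winning team to every controller when time expires.
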(event `MakeSpectator`
  (params (controller :type "/Game/MultiplayerShooterEngine/Blueprints/BP_PlayerController Object Reference"))
  (bind _returnvalue (`|SpawnActorFromClass` "/Game/MultiplayerShooterEngine/Blueprints/BP_Spectator.BP_Spectator_C" (`KismetMathLibrary.MakeTransform` (0.0 0.0 0.0)) "Undefined" "OverrideRootScale" null null))
  (`Controller.Possess` controller _returnvalue)
  (`SceneComponent.K2_SetRelativeLocationAndRotation` :`self` (`self.DefaultSceneRoot`) :`bTeleport` true))

(event `PlayerDied`
  (params (playerController :type "Controller Object Reference") (character :type "Character Object Reference"))
  (bind _asbp_player_state (cast `/Game/MultiplayerShooterEngine/Blueprints/BP_PlayerState` (`Controller.PlayerState` playerController) :!pure true))
  (bind _return (`/Game/MultiplayerShooterEngine/Blueprints/BP_PlayerState.Get Player Display Name` (cast `/Game/MultiplayerShooterEngine/Blueprints/BP_PlayerState` (`Controller.PlayerState` playerController) :!pure true)))
  (`|ExecutionSequence`
    (:`then_0`
      (if (not (`self.warmUp`))
        (bind _asbp_player_base (cast `/Game/MultiplayerShooterEngine/Blueprints/BP_PlayerBase` character))
        (bind _lasthit (`/Game/MultiplayerShooterEngine/Blueprints/BP_PlayerBase.LastHit` _asbp_player_base))
        (`/Engine/EditorBlueprintResources/StandardMacros.IsValid` _lasthit
          (:`Is Valid`
            (bind _asbp_player_state_2 (cast `/Game/MultiplayerShooterEngine/Blueprints/BP_PlayerState` (`Controller.PlayerState` _lasthit)))
            (if (not (== (`/Game/MultiplayerShooterEngine/Blueprints/BP_PlayerState.Team` _asbp_player_state_2) (`/Game/MultiplayerShooterEngine/Blueprints/BP_PlayerState.Team` _asbp_player_state)))
              (`/Game/MultiplayerShooterEngine/Blueprints/BP_PlayerState.AddScore` _asbp_player_state_2 100)
              (if (`/Game/MultiplayerShooterEngine/Blueprints/BP_PlayerBase.LastHeadShot` _asbp_player_base)
                (`/Game/MultiplayerShooterEngine/Blueprints/BP_PlayerState.AddScore` _asbp_player_state_2 50))
              (`/Game/MultiplayerShooterEngine/Blueprints/BP_PlayerState.AddKills` _asbp_player_state_2 1)
              (`/Game/MultiplayerShooterEngine/Blueprints/BP_PlayerState.AddDeath` _asbp_player_state 1)
              (if (== (`/Game/MultiplayerShooterEngine/Blueprints/BP_PlayerState.Team` _asbp_player_state) 0)
                (`/Engine/EditorBlueprintResources/StandardMacros.IncrementInt` (`self.TeamAScore`))
                (else
                  (`/Engine/EditorBlueprintResources/StandardMacros.IncrementInt` (`self.TeamBScore`)))))))))
    (:`then_1`
      (bind _asbp_player_base_2 (cast `/Game/MultiplayerShooterEngine/Blueprints/BP_PlayerBase` character))
      (bind _outactors (`GameplayStatics.GetAllActorsOfClass` "/Game/MultiplayerShooterEngine/Blueprints/BP_PlayerController.BP_PlayerController_C"))
      (for _array_element _outactors
        (bind _lasthit_2 (`/Game/MultiplayerShooterEngine/Blueprints/BP_PlayerBase.LastHit` _asbp_player_base_2))
        (bind _lasthitweaponname (`/Game/MultiplayerShooterEngine/Blueprints/BP_PlayerBase.lastHitWeaponName` _asbp_player_base_2))
        (if (and (`KismetSystemLibrary.IsValid` _lasthit_2) (not (`KismetStringLibrary.EqualEqual_StrStr` _lasthitweaponname)))
          (`/Game/MultiplayerShooterEngine/Blueprints/BP_PlayerController.PrintKillFeed` _array_element (`/Game/MultiplayerShooterEngine/Blueprints/BP_PlayerState.Get Player Display Name` (cast `/Game/MultiplayerShooterEngine/Blueprints/BP_PlayerState` (`Controller.PlayerState` _lasthit_2) :!pure true)) _return _lasthitweaponname false)
          (else
            (`/Game/MultiplayerShooterEngine/Blueprints/BP_PlayerController.PrintKillFeed` _array_element "" _return "Suicide" false)))))
    (:`then_2`
      (`Controller.UnPossess` playerController)
      (bind _asbp_player_base_3 (cast `/Game/MultiplayerShooterEngine/Blueprints/BP_PlayerBase` character)
        (:`then`
          (`/Game/MultiplayerShooterEngine/Blueprints/BP_PlayerBase.DestroyWithDelay` _asbp_player_base_3 3.0))
        (:`CastFailed`
          (`self.K2_DestroyActor` character)))
      (`self.SpawnPlayer` playerController))))

(event `self.ReceiveTick`
  (params (DeltaSeconds :type "Float (single-precision)"))
  (bind _out (`self.SortPlayersByScore` (`self.TeamA`)))
  (set `self.ScoreA` _out)
  (bind _out_2 (`self.SortPlayersByScore` (`self.TeamB`)))
  (set `self.ScoreB` _out_2)
  (`self.Timer`))

(event `Timer`
  (bind _output_get (set `self.Time` (+ (stale _output_get) (`GameplayStatics.GetWorldDeltaSeconds`))))
  (bind (_returnvalue_days _returnvalue_hours _returnvalue_minutes) (`KismetMathLibrary.BreakTimespan` (`KismetMathLibrary.FromSeconds` _output_get)))
  (if (< _returnvalue_minutes (`self.EndTime`))
    (`self.TimerUpdate` _output_get)
    (else
      (`/Engine/EditorBlueprintResources/StandardMacros.DoOnce` false
        (:`Completed`
          (`self.TeamWonMsg` (`KismetMathLibrary.Conv_IntToByte` (`KismetMathLibrary.SelectInt` 0 1 (< (`self.TeamBScore`) (`self.TeamAScore`))))))))))

(event `OnPlayerJoin`
  (params (controller :type "Controller Object Reference"))
  (bind _returnvalue (`Controller.K2_GetPawn` controller))
  (bind _asbp_player_state (cast `/Game/MultiplayerShooterEngine/Blueprints/BP_PlayerState` (`Controller.PlayerState` controller) :!pure true))
  (bind _asbp_player_state_2 (cast `/Game/MultiplayerShooterEngine/Blueprints/BP_PlayerState` (`Controller.PlayerState` controller) :!pure true))
  (`|ExecutionSequence`
    (:`then_0`
      (`|ExecutionSequence`
        (:`then_0`
          (if (== (`KismetArrayLibrary.Array_Length` (`self.TeamA`)) (`KismetArrayLibrary.Array_Length` (`self.TeamB`)))
            (set `/Game/MultiplayerShooterEngine/Blueprints/BP_PlayerState.Team` 0 _asbp_player_state_2)
            (else
              (set `/Game/MultiplayerShooterEngine/Blueprints/BP_PlayerState.Team` (select `bool` (> (`KismetArrayLibrary.Array_Length` (`self.TeamA`)) (`KismetArrayLibrary.Array_Length` (`self.TeamB`))) :`true` 1 :!type "Byte") _asbp_player_state_2))))
        (:`then_1`
          (if (== (`/Game/MultiplayerShooterEngine/Blueprints/BP_PlayerState.Team` _asbp_player_state) 0)
            (`KismetArrayLibrary.Array_AddUnique` (`self.TeamA`) _asbp_player_state)
            (else
              (`KismetArrayLibrary.Array_AddUnique` (`self.TeamB`) _asbp_player_state))))))
    (:`then_1`
      (`/Engine/EditorBlueprintResources/StandardMacros.IsValid` _returnvalue
        (:`Is Valid`
          (`self.K2_DestroyActor` _returnvalue))
        (:`Is Not Valid`
          _))
      (`self.SpawnPlayer` controller))
    (:`then_2`
      (`/Engine/EditorBlueprintResources/StandardMacros.DoOnce` false
        (:`Completed`
          (`self.Timer`))))))

(event `RoundStart`)

(event `TeamWonMsg`
  (params (team :type Byte))
  (bind _outactors (`GameplayStatics.GetAllActorsOfClass` "/Game/MultiplayerShooterEngine/Blueprints/BP_PlayerController.BP_PlayerController_C"))
  (for _array_element _outactors
    (`/Game/MultiplayerShooterEngine/Blueprints/BP_PlayerController.TeamWonMsg` _array_element team)))

(event `self.K2_OnLogout`
  (params (ExitingController :type "Controller Object Reference"))
  (bind _playerstate (`Controller.PlayerState` ExitingController))
  (`/Engine/EditorBlueprintResources/StandardMacros.IsValid` _playerstate
    (:`Is Valid`
      (bind _asbp_player_state (cast `/Game/MultiplayerShooterEngine/Blueprints/BP_PlayerState` _playerstate))
      (`KismetArrayLibrary.Array_RemoveItem` (select `byte` (`/Game/MultiplayerShooterEngine/Blueprints/BP_PlayerState.Team` _asbp_player_state) :`0` (`self.TeamA`) :`1` (`self.TeamB`)) _asbp_player_state))))

(event `ClearLevel`
  (bind _outactors (`GameplayStatics.GetAllActorsOfClassWithTag` "/Script/Engine.Actor" "round"))
  (for _array_element _outactors
    (`self.K2_DestroyActor` _array_element)))

(event `SpawnPlayer`
  (params (controller :type "Controller Object Reference"))
  (bind _team (`/Game/MultiplayerShooterEngine/Blueprints/BP_PlayerState.Team` (cast `/Game/MultiplayerShooterEngine/Blueprints/BP_PlayerState` (`Controller.PlayerState` controller) :!pure true)))
  (bind _outactors (`GameplayStatics.GetAllActorsOfClassWithTag` "/Script/Engine.PlayerStart" (`KismetStringLibrary.Conv_StringToName` (select `byte` _team :`0` "A" :`1` "B"))))
  (bind (_returnvalue_location _returnvalue_rotation) (`KismetMathLibrary.BreakTransform` (`self.GetTransform` (`KismetArrayLibrary.Array_RandomFromStream` _outactors (`self.randomStream`)))))
  (bind _returnvalue (`|SpawnActorFromClass` "/Game/MultiplayerShooterEngine/Blueprints/BP_PlayerBase.BP_PlayerBase_C" (`KismetMathLibrary.MakeTransform` _returnvalue_location _returnvalue_rotation) "AlwaysSpawn" "MultiplyWithRoot" null null))
  (set `/Game/MultiplayerShooterEngine/Blueprints/BP_PlayerBase.team` _team _returnvalue)
  (`Controller.Possess` controller _returnvalue)
  (`/Game/MultiplayerShooterEngine/Blueprints/BP_PlayerBase.SetRotation` _returnvalue _returnvalue_rotation)
  (bind _returnvalue_2 (- _returnvalue_location (0.0 0.0 2000.0)))
  (bind _returnvalue_3 (`|SpawnActorFromClass` "/Game/MultiplayerShooterEngine/Blueprints/Weapons/AK/BP_KA_ProjectileTest.BP_KA_ProjectileTest_C" (`KismetMathLibrary.MakeTransform` _returnvalue_2) "AlwaysSpawn" "OverrideRootScale" null false true false null))
  (bind _slots (`/Game/MultiplayerShooterEngine/Blueprints/BP_PlayerBase.Slots` _returnvalue))
  (`KismetArrayLibrary.Array_Set` _slots 0 _returnvalue_3 true)
  (bind _returnvalue_4 (`|SpawnActorFromClass` "/Game/MultiplayerShooterEngine/Blueprints/Weapons/ShotGun/Shotgun.Shotgun_C" (`KismetMathLibrary.MakeTransform` _returnvalue_2) "AlwaysSpawn" "OverrideRootScale" null false true false null))
  (`KismetArrayLibrary.Array_Set` _slots 1 _returnvalue_4 true))

(fn `SortPlayersByScore`
  (params (States :type "Array of /Game/MultiplayerShooterEngine/Blueprints/BP_PlayerState Object Reference"))
  (returns (Out :type "Array of /Game/MultiplayerShooterEngine/Blueprints/BP_PlayerScore Structure"))
  (locals (Sorted :type Boolean :default true) (ScoreOut :type "Array of /Game/MultiplayerShooterEngine/Blueprints/BP_PlayerScore Structure"))
  (bind _states (`local.States`))
  (if (`local.Sorted`) :!label _label
    (set `local.Sorted` false)
    (for _index (range 1 (+ (`KismetArrayLibrary.Array_LastIndex` States) 1))
      (bind _returnvalue (- _index 1))
      (if (> (`/Game/MultiplayerShooterEngine/Blueprints/BP_PlayerState.PlayerScore` (`|GetArrayItem` _states _index)) (`/Game/MultiplayerShooterEngine/Blueprints/BP_PlayerState.PlayerScore` (`|GetArrayItem` _states _returnvalue)))
        (`KismetArrayLibrary.Array_Swap` (`local.States`) _index _returnvalue)
        (set `local.Sorted` true)))
    (goto _label)
    (else
      (for _array_element (`local.States`)
        (`KismetArrayLibrary.Array_Add` (`local.ScoreOut`) (make `/Game/MultiplayerShooterEngine/Blueprints/BP_PlayerScore` (`/Game/MultiplayerShooterEngine/Blueprints/BP_PlayerState.Get Player Display Name` _array_element) (`/Game/MultiplayerShooterEngine/Blueprints/BP_PlayerState.PlayerScore` _array_element) (`/Game/MultiplayerShooterEngine/Blueprints/BP_PlayerState.kills` _array_element) (`/Game/MultiplayerShooterEngine/Blueprints/BP_PlayerState.death` _array_element) 0 (`KismetMathLibrary.FTrunc` (`PlayerState.GetPingInMilliseconds` _array_element)))))
      (return (`local.ScoreOut`)))))

(fn `UserConstructionScript`)