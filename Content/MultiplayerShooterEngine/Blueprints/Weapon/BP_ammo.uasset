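; BP_ammo is an ammo pickup that adds rounds to the player who uses it.
; Use adds AmmoCount to the slot indexed by AmmoType in the player's Ammo array, then destroys the actor.
; CanUse and GetProgress are stubs that always return false and zero, and Use itself performs no checks or capacity clamping.
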(event `self.Use`
  (params (player :type "/Game/MultiplayerShooterEngine/Blueprints/BP_PlayerBase Object Reference"))
  (bind _ammotype (`self.ammoType`))
  (bind _ammo (`/Game/MultiplayerShooterEngine/Blueprints/BP_PlayerBase.ammo` player))
  (`KismetArrayLibrary.Array_Set` _ammo _ammotype (+ (`|GetArrayItem` _ammo _ammotype) (`self.AmmoCount`)))
  (`self.K2_DestroyActor`))

(fn `CanUse`
  (returns (out :type Boolean))
  (return false))

(fn `GetProgress`
  (returns (out :type "Float (double-precision)"))
  (return 0.0))

(fn `UserConstructionScript`)