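; Player state for the multiplayer shooter that holds a player's score, kills and deaths.
; Simple functions add a given value to each counter, with no authority checks or other logic.
; The display name getter always returns the player name, as its "[AI]" alternative is hardwired off.
; BeginPlay and Tick are empty, and a leftover name-seeded random ID expression sits unused in the event graph.
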(event `self.ReceiveBeginPlay`)

(fn `AddDeath`
  (params (val :type Integer :default 1))
  (bind _output_get (set `self.death` (+ (stale _output_get) val))))

(fn `AddKills`
  (params (val :type Integer :default 1))
  (bind _output_get (set `self.kills` (+ (stale _output_get) val))))

(fn `AddScore`
  (params (val :type Integer :default 1))
  (bind _output_get (set `self.PlayerScore` (+ (stale _output_get) val))))

(fn `Get Player Display Name`
  (returns (return :type String))
  (return (`KismetMathLibrary.SelectString` (`KismetStringLibrary.Concat_StrStr` "[AI]") (`self.GetPlayerName`))))

(fn `UserConstructionScript`)