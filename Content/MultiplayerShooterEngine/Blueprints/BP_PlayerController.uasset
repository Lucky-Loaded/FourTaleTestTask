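; Player controller for the multiplayer shooter that owns the local HUD, pause menu and match-state values.
; Local controllers create the kill feed and optional score bar after a short delay, plus a hold-Tab scoreboard and Escape/P pause toggle that stops aiming.
; On authority, it copies scores and warm-up state from BP_GM every Tick and binds to its timer.
; Kill feed and team-win events are relayed through dispatchers.
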(event `self.ReceiveBeginPlay`
  (bind _asbp_gm (cast `/Game/MultiplayerShooterEngine/Blueprints/BP_GM` (`GameplayStatics.GetGameMode`) :!pure true))
  (`|ExecutionSequence`
    (:`then_0`
      (`KismetSystemLibrary.Delay` 0.2)
      (if (`self.IsLocalController`)
        (bind _returnvalue (`|CreateWidget` "/Game/MultiplayerShooterEngine/UI/KillFeed.KillFeed_C"))
        (`UserWidget.AddToViewport` _returnvalue 0)
        (if (`self.ScoreBar`)
          (bind _returnvalue_2 (`|CreateWidget` "/Game/MultiplayerShooterEngine/UI/GameScore.GameScore_C"))
          (`UserWidget.AddToViewport` _returnvalue_2 0))))
    (:`then_1`
      (`/Engine/EditorBlueprintResources/ActorMacros.Switch Has Authority`
        (:`Authority`
          (set `self.ScoreBar` (`/Game/MultiplayerShooterEngine/Blueprints/BP_GM.TeamScoreBar` _asbp_gm))
          (add `/Game/MultiplayerShooterEngine/Blueprints/BP_GM.TimerUpdate` _asbp_gm (delegate `UpdateTimer`)))))))

(event `UpdateTimer`
  (params (Time :type "Float (double-precision)"))
  (set `self.Time` Time))

(event `Key|Escape`
  (params (Key :type "Key Structure"))
  (:`Pressed`
    (`/Engine/EditorBlueprintResources/StandardMacros.IsValid` (`self.pauseMenu`) :!label _label
      (:`Is Valid`
        (`/Game/MultiplayerShooterEngine/UI/PauseMenu.Resume` (`self.pauseMenu`)))
      (:`Is Not Valid`
        (bind _returnvalue (`|CreateWidget` "/Game/MultiplayerShooterEngine/UI/PauseMenu.PauseMenu_C"))
        (`UserWidget.AddToViewport` _returnvalue 5)
        (set `self.pauseMenu` _returnvalue)
        (bind _asbp_player_base (cast `/Game/MultiplayerShooterEngine/Blueprints/BP_PlayerBase` (`GameplayStatics.GetPlayerCharacter` 0)))
        (`/Game/MultiplayerShooterEngine/Blueprints/BP_PlayerBase.StopAim` _asbp_player_base)))))

(event `Key|P`
  (params (Key :type "Key Structure"))
  (:`Pressed`
    (goto _label)))

(event `PrintKillFeed`
  (params (killer :type String) (killed :type String) (weapon :type String) (hs :type Boolean))
  (`self.ShowInKillFeed` killer killed weapon hs))

(event `Key|Tab`
  (params (Key :type "Key Structure"))
  (:`Pressed`
    (bind _returnvalue (`|CreateWidget` "/Game/MultiplayerShooterEngine/UI/Score.Score_C"))
    (`UserWidget.AddToViewport` _returnvalue 0))
  (:`Released`
    (`/Engine/EditorBlueprintResources/StandardMacros.IsValid` _returnvalue
      (:`Is Valid`
        (`Widget.RemoveFromParent` _returnvalue)))))

(event `SetPing`
  (params (ping :type Integer))
  (set `self.ping` ping))

(event `self.ReceiveTick`
  (params (DeltaSeconds :type "Float (single-precision)"))
  (bind _asbp_gm (cast `/Game/MultiplayerShooterEngine/Blueprints/BP_GM` (`GameplayStatics.GetGameMode`) :!pure true))
  (`/Engine/EditorBlueprintResources/ActorMacros.Switch Has Authority`
    (:`Authority`
      (set `self.TeamA` (`/Game/MultiplayerShooterEngine/Blueprints/BP_GM.ScoreA` _asbp_gm))
      (set `self.TeamB` (`/Game/MultiplayerShooterEngine/Blueprints/BP_GM.ScoreB` _asbp_gm))
      (set `self.warmUp` (`/Game/MultiplayerShooterEngine/Blueprints/BP_GM.warmUp` _asbp_gm))
      (set `self.TeamAScore` (`/Game/MultiplayerShooterEngine/Blueprints/BP_GM.TeamAScore` _asbp_gm))
      (set `self.TeamBScore` (`/Game/MultiplayerShooterEngine/Blueprints/BP_GM.TeamBScore` _asbp_gm)))))

(event `TeamWonMsg`
  (params (team :type Byte))
  (`self.TeamWon` team))

(fn `UserConstructionScript`)