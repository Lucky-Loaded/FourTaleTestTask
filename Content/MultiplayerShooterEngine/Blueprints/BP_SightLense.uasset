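; BP_SightLense is a sight lens that shows a scene capture view on a cylinder mesh.
; BeginPlay creates a render target, feeds it to the cylinder's dynamic material and moves ticking to PostUpdateWork.
; While enabled, each tick applies the FOV, captures the scene and writes the player camera's position relative to the capture into SightParameterCollection.
; The construction script places the capture at CameraOffset.
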(event `self.ReceiveTick`
  (params (DeltaSeconds :type "Float (single-precision)"))
  (bind _returnvalue_location (`KismetMathLibrary.BreakTransform` (`KismetMathLibrary.MakeRelativeTransform` (`SceneComponent.K2_GetComponentToWorld` (`PlayerCameraManager.TransformComponent` (`GameplayStatics.GetPlayerCameraManager` 0))) (`SceneComponent.K2_GetComponentToWorld` (`self.SceneCaptureComponent2D`)))))
  (if (`self.enabled`)
    (`|ExecutionSequence`
      (:`then_1`
        (set `SceneCaptureComponent2D.FOVAngle` (`self.FOV`) (`self.SceneCaptureComponent2D`))
        (bind _output_get (set `self.RelativeLocation` _returnvalue_location))
        (`SceneCaptureComponent2D.CaptureScene` (`self.SceneCaptureComponent2D`))
        (`KismetMaterialLibrary.SetVectorParameterValue` "/Game/MultiplayerShooterEngine/Materials/SightParameterCollection.SightParameterCollection" "CameraRelativeLocation" (make `LinearColor` (.x _output_get) (.y _output_get) (.z _output_get)))))))

(event `self.ReceiveBeginPlay`
  (bind _textureresolution (`self.TextureResolution`))
  (`self.SetTickGroup` "TG_PostUpdateWork")
  (bind _returnvalue (`KismetRenderingLibrary.CreateRenderTarget2D` _textureresolution _textureresolution))
  (set `self.RT` _returnvalue)
  (bind _returnvalue_2 (`PrimitiveComponent.CreateDynamicMaterialInstance` (`self.Cylinder`) 0 (`self.Material`) "None"))
  (bind _output_get (set `self.MI` _returnvalue_2))
  (`MaterialInstanceDynamic.SetTextureParameterValue` _output_get "RT" (`self.RT`))
  (set `SceneCaptureComponent2D.TextureTarget` (`self.RT`) (`self.SceneCaptureComponent2D`))
  (`KismetMaterialLibrary.SetVectorParameterValue` "/Game/MultiplayerShooterEngine/Materials/SightParameterCollection.SightParameterCollection" "CameraRelativeLocation" (make `LinearColor` -1000000.0 -1000000.0 -1000000.0)))

(fn `UserConstructionScript`
  (bind _scenecapturecomponent2d (`self.SceneCaptureComponent2D`))
  (`SceneComponent.K2_SetRelativeLocation` _scenecapturecomponent2d (`self.CameraOffset`) false false)
  (set `SceneCaptureComponent2D.FOVAngle` (`self.FOV`) _scenecapturecomponent2d))